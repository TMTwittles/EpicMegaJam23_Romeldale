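; Movement component for an AI ship that steers its owner through a looping list of target positions.
; Each tick, acceleration toward the current target scales by previous target's distance from world origin over remaining distance.
; Clamped velocity moves the owner without sweep or delta time, facing it along its motion.
; GenerateTargetPositionsAroundActor builds a debug-drawn ring of points; it, unfinished Hover and empty MoveForward are never called here.
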(event `self.ReceiveBeginPlay`
  (set `self.PreviousTargetPosition` (`Actor.K2_GetActorLocation` (`self.GetOwner`))))

(event `self.ReceiveTick`
  (params (DeltaSeconds :type "Float (single-precision)"))
  (bind _returnvalue (`self.GetOwner`))
  (bind _returnvalue_2 (`Actor.K2_GetActorLocation` _returnvalue))
  (bind _returnvalue_3 (+ _returnvalue_2 (`self.Velocity`)))
  (`self.SteerToTargetPosition`)
  (`Actor.K2_SetActorLocation` _returnvalue _returnvalue_3 false false)
  (`Actor.K2_SetActorRotation` _returnvalue (`KismetMathLibrary.FindLookAtRotation` _returnvalue_2 _returnvalue_3) false))

(fn `CheckGrounded`
  (returns (Grounded :type Boolean) (OutHit :type "HitResult Structure"))
  (bind _returnvalue (`Actor.K2_GetActorLocation` (`self.GetOwner`)))
  (bind (_outhit _returnvalue_2) (`KismetSystemLibrary.LineTraceSingle` :`Start` _returnvalue :`End` (+ _returnvalue (* (0.0 0.0 -1.0) (`self.CheckGroundLineTraceDistance`))) :`TraceChannel` "TraceTypeQuery3" :`DrawDebugType` "ForOneFrame"))
  (return _returnvalue_2 _outhit))

(fn `ClampVectorMagnitude`
  (params (VectorToClamp :type "Vector Structure") (MaxMagnitude :type "Float (double-precision)"))
  (returns (VectorClamped :type "Vector Structure"))
  (bind _returnvalue (`KismetMathLibrary.VSize` VectorToClamp))
  (if (> _returnvalue MaxMagnitude)
    (return (* VectorToClamp (/ MaxMagnitude _returnvalue)))
    (else
      (return VectorToClamp))))

(fn `Generate Target PositionsAroundActor`
  (params (Actor :type "Actor Object Reference") (Radius :type "Float (double-precision)") (NumPoints :type Integer))
  (bind _returnvalue (`Actor.K2_GetActorLocation` Actor))
  (`KismetSystemLibrary.FlushPersistentDebugLines`)
  (`KismetArrayLibrary.Array_Clear` (`self.TargetPositions`))
  (set `self.TargetPositionStepAmountDegrees` (`KismetMathLibrary.Conv_IntToDouble` (/ 360 NumPoints)))
  (bind _output_get (set `self.TargetPositionStepIter` 0.0))
  (set `self.TargetPositionIter` 0)
  (for _ (range (+ NumPoints 1))
    (bind _returnvalue_2 (+ _returnvalue (* (`KismetMathLibrary.RotateAngleAxis` (`Actor.GetActorForwardVector` Actor) _output_get (`Actor.GetActorUpVector` Actor)) Radius)))
    (bind (_outhit _returnvalue_3) (`KismetSystemLibrary.LineTraceSingle` :`Start` _returnvalue :`End` _returnvalue_2 :`TraceChannel` "TraceTypeQuery3" :`DrawDebugType` "Persistent"))
    (if _returnvalue_3
      _
      (else
        _))
    (`KismetArrayLibrary.Array_Add` (`self.TargetPositions`) _returnvalue_2)
    (`KismetSystemLibrary.DrawDebugSphere` _returnvalue_2 100.0 12 (struct :`R` 1.0 :`G` 1.0 :`B` 1.0 :`A` 1.0) 10.0)
    (set `self.TargetPositionStepIter` (+ (`self.TargetPositionStepAmountDegrees`) (`self.TargetPositionStepIter`)))))

(fn `GetNextTargetPosition`
  (returns (TargetPos :type "Vector Structure"))
  (set `self.DistanceToNextPosition` (`KismetMathLibrary.Vector_Distance` (`self.PreviousTargetPosition`)))
  (if (<= (`KismetMathLibrary.Vector_Distance` (`Actor.K2_GetActorLocation` (`self.GetOwner`)) (`|GetArrayItem` (`self.TargetPositions`) (`self.TargetPositionIter`))) (`self.MinDistanceToReachTargetPos`))
    (set `self.PreviousTargetPosition` (`|GetArrayItem` (`self.TargetPositions`) (`self.TargetPositionIter`)))
    (if (>= (`self.TargetPositionIter`) (- (`KismetArrayLibrary.Array_Length` (`self.TargetPositions`)) 1))
      (set `self.TargetPositionIter` 0)
      (else
        (set `self.TargetPositionIter` (+ (`self.TargetPositionIter`) 1)))))
  (return (`|GetArrayItem` (`self.TargetPositions`) (`self.TargetPositionIter`))))

(fn `GetRemainingDistanceToTargetLocation`
  (returns (DistanceToTargetPosition :type "Float (double-precision)"))
  (return (`KismetMathLibrary.Vector_Distance` (`Actor.K2_GetActorLocation` (`self.GetOwner`)))))

(fn `Hover`
  (bind (_velocity_x _velocity_y) (`KismetMathLibrary.BreakVector` (`self.Velocity`)))
  (bind (_returnvalue_x _returnvalue_y _returnvalue_z) (`KismetMathLibrary.BreakVector` (* (0.0 0.0 -1.0) (`self.Gravity`))))
  (bind (_grounded _outhit) (`self.CheckGrounded`))
  (if (not _grounded)
    (set `self.Velocity` (`KismetMathLibrary.MakeVector` _velocity_x _velocity_y _returnvalue_z))))

(fn `MoveForward`)

(fn `SteerToTargetPosition`
  (bind _returnvalue (`Actor.K2_GetActorLocation` (`self.GetOwner`)))
  (bind _targetpos (`self.GetNextTargetPosition`))
  (bind _output_get (set `self.Acceleration` (* (`KismetMathLibrary.Normal` (- _targetpos _returnvalue)) (* (`self.HoverSpeed`) (/ (`self.DistanceToNextPosition`) (`KismetMathLibrary.Vector_Distance` _returnvalue _targetpos))))))
  (set `self.Velocity` (`self.ClampVectorMagnitude` (+ (`self.Velocity`) _output_get) (`self.MaxHoverSpeed`))))