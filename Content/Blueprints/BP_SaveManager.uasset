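; BP_SaveManager autosaves the player's metals, movement stats and chassis, rudder and thruster unlocks to "SaveSlot".
; After BeginPlay, it takes the save object from BP_GameInstance if the slot exists, ignoring its own load result, or creates one otherwise.
; A 30-second Delay loop copies PlayerRef values into both game instance and save object, then writes the slot.
; Weapon cost copying exists but is disconnected.
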(event `self.ReceiveBeginPlay`
  (bind _playerref (`self.PlayerRef`))
  (bind _as_bp_game_instance (`self.As BP Game Instance`))
  (bind _my_save_game_ref (`self.My Save Game Ref`))
  (bind _maxspeed (`/Game/ThirdPerson/Blueprints/BP_ThirdPersonCharacter.MaxSpeed` _playerref))
  (bind _chassis1unlocked (`/Game/ThirdPerson/Blueprints/BP_ThirdPersonCharacter.Chassis1Unlocked` _playerref))
  (bind _chassis2unlocked (`/Game/ThirdPerson/Blueprints/BP_ThirdPersonCharacter.Chassis2Unlocked` _playerref))
  (bind _chassis3unlocked (`/Game/ThirdPerson/Blueprints/BP_ThirdPersonCharacter.Chassis3Unlocked` _playerref))
  (bind _chassis4unlocked (`/Game/ThirdPerson/Blueprints/BP_ThirdPersonCharacter.Chassis4Unlocked` _playerref))
  (bind _ferrousmetals (`/Game/ThirdPerson/Blueprints/BP_ThirdPersonCharacter.FerrousMetals` _playerref))
  (bind _chassis5unlocked (`/Game/ThirdPerson/Blueprints/BP_ThirdPersonCharacter.Chassis5Unlocked` _playerref))
  (bind _chassis6unlocked (`/Game/ThirdPerson/Blueprints/BP_ThirdPersonCharacter.Chassis6Unlocked` _playerref))
  (bind _accelerationrate (`/Game/ThirdPerson/Blueprints/BP_ThirdPersonCharacter.AccelerationRate` _playerref))
  (bind _rudder1unlocked (`/Game/ThirdPerson/Blueprints/BP_ThirdPersonCharacter.Rudder1Unlocked` _playerref))
  (bind _rudder2unlocked (`/Game/ThirdPerson/Blueprints/BP_ThirdPersonCharacter.Rudder2Unlocked` _playerref))
  (bind _rudder3unlocked (`/Game/ThirdPerson/Blueprints/BP_ThirdPersonCharacter.Rudder3Unlocked` _playerref))
  (bind _rudder4unlocked (`/Game/ThirdPerson/Blueprints/BP_ThirdPersonCharacter.Rudder4Unlocked` _playerref))
  (bind _rudder5unlocked (`/Game/ThirdPerson/Blueprints/BP_ThirdPersonCharacter.Rudder5Unlocked` _playerref))
  (bind _rudder6unlocked (`/Game/ThirdPerson/Blueprints/BP_ThirdPersonCharacter.Rudder6Unlocked` _playerref))
  (bind _thruster1unlocked (`/Game/ThirdPerson/Blueprints/BP_ThirdPersonCharacter.Thruster1Unlocked` _playerref))
  (bind _thruster2unlocked (`/Game/ThirdPerson/Blueprints/BP_ThirdPersonCharacter.Thruster2Unlocked` _playerref))
  (bind _thruster3unlocked (`/Game/ThirdPerson/Blueprints/BP_ThirdPersonCharacter.Thruster3Unlocked` _playerref))
  (bind _thruster4unlocked (`/Game/ThirdPerson/Blueprints/BP_ThirdPersonCharacter.Thruster4Unlocked` _playerref))
  (bind _thruster5unlocked (`/Game/ThirdPerson/Blueprints/BP_ThirdPersonCharacter.Thruster5Unlocked` _playerref))
  (bind _thruster6unlocked (`/Game/ThirdPerson/Blueprints/BP_ThirdPersonCharacter.Thruster6Unlocked` _playerref))
  (bind _preciousmetals (`/Game/ThirdPerson/Blueprints/BP_ThirdPersonCharacter.PreciousMetals` _playerref))
  (bind _exoticmetals (`/Game/ThirdPerson/Blueprints/BP_ThirdPersonCharacter.ExoticMetals` _playerref))
  (`KismetSystemLibrary.Delay` 1.0)
  (bind _returnvalue (`GameplayStatics.DoesSaveGameExist` "SaveSlot"))
  (if _returnvalue
    (`GameplayStatics.LoadGameFromSlot` "SaveSlot")
    (bind _asbp_game_instance (cast `/Game/Blueprints/BP_GameInstance` (`GameplayStatics.GetGameInstance`)))
    (set `self.As BP Game Instance` _asbp_game_instance)
    (set `self.My Save Game Ref` (`/Game/Blueprints/BP_GameInstance.MySaveGameRef` _asbp_game_instance))
    (else
      (bind _returnvalue_2 (`GameplayStatics.CreateSaveGameObject` "/Game/Blueprints/MySaveGame.MySaveGame_C"))
      (bind _asbp_game_instance_2 (cast `/Game/Blueprints/BP_GameInstance` (`GameplayStatics.GetGameInstance`)))
      (set `self.As BP Game Instance` _asbp_game_instance_2)
      (set `self.My Save Game Ref` _returnvalue_2)))
  (`KismetSystemLibrary.Delay` 30.0 :!label _label)
  (`KismetSystemLibrary.PrintString` "Saving")
  (set `/Game/Blueprints/BP_GameInstance.FerrousMetals` _ferrousmetals _as_bp_game_instance)
  (set `/Game/Blueprints/MySaveGame.FerrousMetals` _ferrousmetals _my_save_game_ref)
  (set `/Game/Blueprints/BP_GameInstance.PreciousMetals` _preciousmetals _as_bp_game_instance)
  (set `/Game/Blueprints/MySaveGame.PreciousMetals` _preciousmetals _my_save_game_ref)
  (set `/Game/Blueprints/MySaveGame.ExoticMetals` _exoticmetals _my_save_game_ref)
  (set `/Game/Blueprints/BP_GameInstance.ExoticMetals` _exoticmetals _as_bp_game_instance)
  (set `/Game/Blueprints/MySaveGame.MaxSpeed` _maxspeed _my_save_game_ref)
  (set `/Game/Blueprints/BP_GameInstance.MaxSpeed` _maxspeed _as_bp_game_instance)
  (set `/Game/Blueprints/BP_GameInstance.Chassis1Unlocked` _chassis1unlocked _as_bp_game_instance)
  (set `/Game/Blueprints/MySaveGame.Chassis1Unlocked` _chassis1unlocked _my_save_game_ref)
  (set `/Game/Blueprints/MySaveGame.Chassis2Unlocked` _chassis2unlocked _my_save_game_ref)
  (set `/Game/Blueprints/BP_GameInstance.Chassis2Unlocked` _chassis2unlocked _as_bp_game_instance)
  (set `/Game/Blueprints/BP_GameInstance.Chassis3Unlocked` _chassis3unlocked _as_bp_game_instance)
  (set `/Game/Blueprints/MySaveGame.Chassis3Unlocked` _chassis3unlocked _my_save_game_ref)
  (set `/Game/Blueprints/MySaveGame.Chassis4Unlocked` _chassis4unlocked _my_save_game_ref)
  (set `/Game/Blueprints/BP_GameInstance.Chassis4Unlocked` _chassis4unlocked _as_bp_game_instance)
  (set `/Game/Blueprints/BP_GameInstance.Chassis5Unlocked` _chassis5unlocked _as_bp_game_instance)
  (set `/Game/Blueprints/MySaveGame.Chassis5Unlocked` _chassis5unlocked _my_save_game_ref)
  (set `/Game/Blueprints/MySaveGame.Chassis6Unlocked` _chassis6unlocked _my_save_game_ref)
  (set `/Game/Blueprints/BP_GameInstance.Chassis6Unlocked` _chassis6unlocked _as_bp_game_instance)
  (set `/Game/Blueprints/MySaveGame.AccelerationRate` _accelerationrate _my_save_game_ref)
  (set `/Game/Blueprints/BP_GameInstance.AccelerationRate` _accelerationrate _as_bp_game_instance)
  (set `/Game/Blueprints/MySaveGame.Rudder1Unlocked` _rudder1unlocked _my_save_game_ref)
  (set `/Game/Blueprints/BP_GameInstance.Rudder1Unlocked` _rudder1unlocked _as_bp_game_instance)
  (set `/Game/Blueprints/MySaveGame.Rudder2Unlocked` _rudder2unlocked _my_save_game_ref)
  (set `/Game/Blueprints/BP_GameInstance.Rudder2Unlocked` _rudder2unlocked _as_bp_game_instance)
  (set `/Game/Blueprints/MySaveGame.Rudder3Unlocked` _rudder3unlocked _my_save_game_ref)
  (set `/Game/Blueprints/BP_GameInstance.Rudder3Unlocked` _rudder3unlocked _as_bp_game_instance)
  (set `/Game/Blueprints/BP_GameInstance.Rudder4Unlocked` _rudder4unlocked _as_bp_game_instance)
  (set `/Game/Blueprints/MySaveGame.Rudder4Unlocked` _rudder4unlocked _my_save_game_ref)
  (set `/Game/Blueprints/MySaveGame.Rudder5Unlocked` _rudder5unlocked _my_save_game_ref)
  (set `/Game/Blueprints/BP_GameInstance.Rudder5Unlocked` _rudder5unlocked _as_bp_game_instance)
  (set `/Game/Blueprints/BP_GameInstance.Rudder6Unlocked` _rudder6unlocked _as_bp_game_instance)
  (set `/Game/Blueprints/MySaveGame.Rudder6Unlocked` _rudder6unlocked _my_save_game_ref)
  (set `/Game/Blueprints/MySaveGame.Thruster1Unlocked` _thruster1unlocked _my_save_game_ref)
  (set `/Game/Blueprints/BP_GameInstance.Thruster1Unlocked` _thruster1unlocked _as_bp_game_instance)
  (set `/Game/Blueprints/BP_GameInstance.Thruster2Unlocked` _thruster2unlocked _as_bp_game_instance)
  (set `/Game/Blueprints/MySaveGame.Thruster2Unlocked` _thruster2unlocked _my_save_game_ref)
  (set `/Game/Blueprints/BP_GameInstance.Thruster3Unlocked` _thruster3unlocked _as_bp_game_instance)
  (set `/Game/Blueprints/MySaveGame.Thruster3Unlocked` _thruster3unlocked _my_save_game_ref)
  (set `/Game/Blueprints/BP_GameInstance.Thruster4Unlocked` _thruster4unlocked _as_bp_game_instance)
  (set `/Game/Blueprints/MySaveGame.Thruster4Unlocked` _thruster4unlocked _my_save_game_ref)
  (set `/Game/Blueprints/BP_GameInstance.Thruster5Unlocked` _thruster5unlocked _as_bp_game_instance)
  (set `/Game/Blueprints/MySaveGame.Thruster5Unlocked` _thruster5unlocked _my_save_game_ref)
  (set `/Game/Blueprints/BP_GameInstance.Thruster6Unlocked` _thruster6unlocked _as_bp_game_instance)
  (set `/Game/Blueprints/MySaveGame.Thruster6Unlocked` _thruster6unlocked _my_save_game_ref)
  (`GameplayStatics.SaveGameToSlot` (`self.My Save Game Ref`) "SaveSlot")
  (goto _label))

(fn `UserConstructionScript`)