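; BP_ScrapFerrous is a ferrous metal scrap pickup that the third-person character collects by overlapping its HitBox.
; Collection adds a random amount to FerrousMetals on the character and game instance, plays a sound, then destroys the actor.
; It also writes the game instance total plus another random amount to the save object and saves immediately.
; Each random amount is rolled separately, so the three counts can diverge.
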(event `self.HitBox.OnComponentBeginOverlap`
  (params (OverlappedComponent :type "PrimitiveComponent Object Reference") (OtherActor :type "Actor Object Reference") (OtherComp :type "PrimitiveComponent Object Reference") (OtherBodyIndex :type Integer) (bFromSweep :type Boolean) (SweepResult :type "HitResult Structure (by ref)"))
  (bind _returnvalue (`KismetMathLibrary.RandomIntegerInRange` 25 40))
  (bind _asbp_third_person_character (cast `/Game/ThirdPerson/Blueprints/BP_ThirdPersonCharacter` OtherActor))
  (set `/Game/ThirdPerson/Blueprints/BP_ThirdPersonCharacter.FerrousMetals` (+ (`/Game/ThirdPerson/Blueprints/BP_ThirdPersonCharacter.FerrousMetals` _asbp_third_person_character) _returnvalue) _asbp_third_person_character)
  (`GameplayStatics.PlaySound2D` "/Game/Audio/SFX_FerrousMetal_Cue.SFX_FerrousMetal_Cue" 1.0 1.0 0.0 null null)
  ;[0.02604 0.02604 0.02604] Game Instance & Save Game referencing
  (`|ExecutionSequence`
    (:`then_0`
      (bind _asbp_game_instance (cast `/Game/Blueprints/BP_GameInstance` (`GameplayStatics.GetGameInstance`)))
      (bind _returnvalue_2 (+ (`/Game/Blueprints/BP_GameInstance.FerrousMetals` _asbp_game_instance) _returnvalue))
      (set `/Game/Blueprints/BP_GameInstance.FerrousMetals` _returnvalue_2 _asbp_game_instance)
      (bind _mysavegameref (`/Game/Blueprints/BP_GameInstance.MySaveGameRef` _asbp_game_instance))
      (set `/Game/Blueprints/MySaveGame.FerrousMetals` _returnvalue_2 _mysavegameref)
      (`GameplayStatics.SaveGameToSlot` _mysavegameref "SaveSlot"))
    (:`then_1`
      (`self.K2_DestroyActor`))))

(fn `UserConstructionScript`)