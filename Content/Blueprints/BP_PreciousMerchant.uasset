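; BP_PreciousMerchant is a merchant actor that shows the WB_PreciousMerchantStore widget when the player character overlaps its collision box.
; Begin overlap calls OpenWidget directly, which, guarded by range and open-state flags, disables movement, shows the cursor and focuses the store.
; End overlap removes the widget and restores game-only input and walking movement.
; Interact-prompt and older close logic remain as disconnected legacy nodes.
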(event `OpenWidget`
  (bind _returnvalue (`GameplayStatics.GetPlayerController` 0))
  ;[0.02604 0.02604 0.02604] Open widget when the player is in range and pressed 'E'
  (if (`self.IsInWidget?`)
    _
    (elif (`self.PlayerInRange?`)
      (set `self.IsInWidget?` true)
      (bind _asbp_third_person_character (cast `/Game/ThirdPerson/Blueprints/BP_ThirdPersonCharacter` (`GameplayStatics.GetPlayerCharacter` 0)))
      (`CharacterMovementComponent.DisableMovement` (`Character.CharacterMovement` _asbp_third_person_character))
      (bind _returnvalue_2 (`|CreateWidget` "/Game/UI/WB_PreciousMerchantStore.WB_PreciousMerchantStore_C"))
      (bind _output_get (set `self.BuyItemWidget` _returnvalue_2))
      (`UserWidget.AddToViewport` _output_get 0)
      (set `PlayerController.bShowMouseCursor` true _returnvalue)
      (`WidgetBlueprintLibrary.SetInputMode_GameAndUIEx` _returnvalue (`self.BuyItemWidget`)))))

(event `self.CollisionBox.OnComponentBeginOverlap`
  (params (OverlappedComponent :type "PrimitiveComponent Object Reference") (OtherActor :type "Actor Object Reference") (OtherComp :type "PrimitiveComponent Object Reference") (OtherBodyIndex :type Integer) (bFromSweep :type Boolean) (SweepResult :type "HitResult Structure (by ref)"))
  ;[0.02604 0.02288 0] Handles instructional text on overlapping collision box area (Somehow not fucking working for no fucking reason :) )
  (cast `/Game/ThirdPerson/Blueprints/BP_ThirdPersonCharacter` OtherActor)
  (set `self.PlayerInRange?` true)
  (`self.OpenWidget`)
  (set `self.IsInWidget?` true))

(event `self.CollisionBox.OnComponentEndOverlap`
  (params (OverlappedComponent :type "PrimitiveComponent Object Reference") (OtherActor :type "Actor Object Reference") (OtherComp :type "PrimitiveComponent Object Reference") (OtherBodyIndex :type Integer))
  (bind _returnvalue (`GameplayStatics.GetPlayerController` 0))
  ;[0.02604 0.02288 0] Handles instructional text on overlapping collision box area (Somehow not fucking working for no fucking reason :) )
  (cast `/Game/ThirdPerson/Blueprints/BP_ThirdPersonCharacter` OtherActor)
  (set `self.PlayerInRange?` false)
  (`Widget.RemoveFromParent` (`self.BuyItemWidget`))
  (set `PlayerController.bShowMouseCursor` false _returnvalue)
  (`WidgetBlueprintLibrary.SetInputMode_GameOnly` _returnvalue)
  (`CharacterMovementComponent.SetMovementMode` (`Character.CharacterMovement` (stale `OpenWidget` _asbp_third_person_character)) "MOVE_Walking" 0)
  (set `self.IsInWidget?` false))

(fn `UserConstructionScript`)