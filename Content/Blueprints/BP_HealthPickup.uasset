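; BP_HealthPickup is a pickup that restores a small random amount of health to the third-person player character.
; When the character overlaps its HitBox, it raises current health, clamped to the character's maximum, and plays a 2D sound.
; It then copies the game instance's FerrousMetals count, with zero added, into the save object, saves to a slot, and destroys itself.
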(event `self.HitBox.OnComponentBeginOverlap`
  (params (OverlappedComponent :type "PrimitiveComponent Object Reference") (OtherActor :type "Actor Object Reference") (OtherComp :type "PrimitiveComponent Object Reference") (OtherBodyIndex :type Integer) (bFromSweep :type Boolean) (SweepResult :type "HitResult Structure (by ref)"))
  (bind _asbp_third_person_character (cast `/Game/ThirdPerson/Blueprints/BP_ThirdPersonCharacter` OtherActor))
  (set `/Game/ThirdPerson/Blueprints/BP_ThirdPersonCharacter.CurrentPlayerHealth` (`KismetMathLibrary.FClamp` (+ (`/Game/ThirdPerson/Blueprints/BP_ThirdPersonCharacter.CurrentPlayerHealth` _asbp_third_person_character) (`KismetMathLibrary.RandomFloatInRange` 5.0 10.0)) 0.0 (`/Game/ThirdPerson/Blueprints/BP_ThirdPersonCharacter.MaxPlayerHealth` _asbp_third_person_character)) _asbp_third_person_character)
  (`GameplayStatics.PlaySound2D` "/Game/Audio/SFX_HealthPickup.SFX_HealthPickup" 1.0 1.0 0.0 null null)
  ;[0.02604 0.02604 0.02604] Game Instance & Save Game referencing
  (`|ExecutionSequence`
    (:`then_0`
      (bind _asbp_game_instance (cast `/Game/Blueprints/BP_GameInstance` (`GameplayStatics.GetGameInstance`)))
      (bind _returnvalue (+ (`/Game/Blueprints/BP_GameInstance.FerrousMetals` _asbp_game_instance) 0))
      (set `/Game/Blueprints/BP_GameInstance.FerrousMetals` _returnvalue _asbp_game_instance)
      (bind _mysavegameref (`/Game/Blueprints/BP_GameInstance.MySaveGameRef` _asbp_game_instance))
      (set `/Game/Blueprints/MySaveGame.FerrousMetals` _returnvalue _mysavegameref)
      (`GameplayStatics.SaveGameToSlot` _mysavegameref "SaveSlot"))
    (:`then_1`
      (`self.K2_DestroyActor`))))

(fn `UserConstructionScript`)