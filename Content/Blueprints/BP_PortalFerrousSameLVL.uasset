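; BP_PortalFerrousSameLVL is a trigger portal that teleports the player character to the Ferrous merchant within the same level.
; On Box overlap by BP_ThirdPersonCharacter, it averages the locations of all BP_FerrousMerchant actors and moves the character there with a fixed Y offset.
; A WB_Fade widget is added and removed around the teleport with no delay, then a second one plays the reverse fade.
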(event `self.Box.OnComponentBeginOverlap`
  (params (OverlappedComponent :type "PrimitiveComponent Object Reference") (OtherActor :type "Actor Object Reference") (OtherComp :type "PrimitiveComponent Object Reference") (OtherBodyIndex :type Integer) (bFromSweep :type Boolean) (SweepResult :type "HitResult Structure (by ref)"))
  (bind _asbp_third_person_character (cast `/Game/ThirdPerson/Blueprints/BP_ThirdPersonCharacter` OtherActor))
  (bind _returnvalue (`|CreateWidget` "/Game/UI/WB_Fade.WB_Fade_C"))
  (`UserWidget.AddToViewport` _returnvalue 0)
  (bind _outactors (`GameplayStatics.GetAllActorsOfClass` "/Game/Blueprints/BP_FerrousMerchant.BP_FerrousMerchant_C"))
  (bind _returnvalue_2 (`GameplayStatics.GetActorArrayAverageLocation` _outactors))
  (`self.K2_SetActorLocation` _asbp_third_person_character (`KismetMathLibrary.MakeVector` (.x _returnvalue_2) (+ (.y _returnvalue_2) 1500.0) (.z _returnvalue_2)) false true)
  (`Widget.RemoveFromParent` _returnvalue)
  (bind _returnvalue_3 (`|CreateWidget` "/Game/UI/WB_Fade.WB_Fade_C"))
  (`/Game/UI/WB_Fade.ReverseFadeAnim` _returnvalue_3)
  (`UserWidget.AddToViewport` _returnvalue_3 0))

(fn `UserConstructionScript`)