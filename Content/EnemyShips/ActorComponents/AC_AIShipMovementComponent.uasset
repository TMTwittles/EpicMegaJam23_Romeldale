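; Actor component that moves an AI enemy ship by applying physics to its root primitive component each tick.
; Horizontal seek steering toward a set target position produces a clamped acceleration force, while a velocity-change impulse provides hover lift.
; Lift weakens with distance along a downward trace, whose randomized length follows player height, with a fallback for ships below the player.
; CalculateForwardForce is defined but never called here.
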(event `self.ReceiveTick`
  (params (DeltaSeconds :type "Float (single-precision)"))
  (bind _rootprimitivecomponent (`self.GetRootPrimiitiveComponent`))
  (`self.CalculateSteeringForce`)
  (`self.CalculateUpdwardsForce`)
  (`PrimitiveComponent.AddForce` _rootprimitivecomponent (`self.SteeringForce`) "None" true)
  (`PrimitiveComponent.AddImpulse` _rootprimitivecomponent (`self.UpdwardsForce`) "None" true))

(fn `CalculateForwardForce`
  (if (`self.ValidTargetPosition`)
    (set `self.ForwardForce` (* (`Actor.GetActorForwardVector` (`self.GetOwner`)) (`self.ForwardForceAmount`)))
    (else
      (set `self.ForwardForce` (0.0 0.0 0.0)))))

(fn `CalculateSteeringForce`
  (if (`self.ValidTargetPosition`)
    (bind _output_get (set `self.DesiredVelocity` (* (* (`KismetMathLibrary.Normal` (- (`self.TargetPosition`) (`Actor.K2_GetActorLocation` (`self.GetOwner`)))) (`self.MaxSpeed`)) (1.0 1.0 0.0))))
    (set `self.SteeringForce` (`self.ClampVectorMagnitude` (- _output_get (`SceneComponent.GetComponentVelocity` (`self.GetRootPrimiitiveComponent`))) (`self.MaxSteeringForce`)))
    (else
      (set `self.SteeringForce` (0.0 0.0 0.0)))))

(fn `CalculateUpdwardsForce`
  (bind (_grounded _distancefromground) (`self.ComponentGrounded`))
  (if _grounded
    (set `self.UpdwardsForce` (* (`self.UpdwardsForceDirection`) (* (`self.UpdwardsForceAmount`) (- 1.0 (/ _distancefromground (`self.LineTraceDistance`))))))
    (else
      (set `self.UpdwardsForce` (0.0 0.0 0.0)))))

(fn `ClampVectorMagnitude`
  (params (VectorToClamp :type "Vector Structure") (MaxMagnitude :type "Float (double-precision)"))
  (returns (VectorClamped :type "Vector Structure"))
  (bind _returnvalue (`KismetMathLibrary.VSize` VectorToClamp))
  (if (> _returnvalue MaxMagnitude)
    (return (* VectorToClamp (/ MaxMagnitude _returnvalue)))
    (else
      (return VectorToClamp))))

(fn `ComponentGrounded`
  (returns (Grounded :type Boolean) (DistanceFromGround :type "Float (double-precision)"))
  (bind _returnvalue (`self.GetOwner`))
  (bind (_returnvalue_x _returnvalue_y _returnvalue_z) (`KismetMathLibrary.BreakVector` (`Actor.K2_GetActorLocation` (`self.GetOwner`))))
  (bind _returnvalue_2 (`Actor.K2_GetActorLocation` _returnvalue))
  (bind (_returnvalue_x_2 _returnvalue_y_2 _returnvalue_z_2) (`KismetMathLibrary.BreakVector` (`Actor.K2_GetActorLocation` (`GameplayStatics.GetPlayerCharacter` 0))))
  (`self.Update Line Trace Distance`)
  (bind (_outhit _returnvalue_3) (`KismetSystemLibrary.LineTraceSingle` _returnvalue_2 (+ _returnvalue_2 (`KismetMathLibrary.MakeVector` 0.0 0.0 (* -1.0 (`self.LineTraceDistance`)))) "TraceTypeQuery1" false (`|MakeArray` _returnvalue)))
  (if _returnvalue_3
    (return true (`.Distance` (`GameplayStatics.BreakHitResult` _outhit)))
    (elif (<= _returnvalue_z _returnvalue_z_2)
      (return true _returnvalue_z_2)
      (else
        (return false 0.0)))))

(fn `GetRootPrimiitiveComponent`
  (returns (RootPrimitiveComponent :type "PrimitiveComponent Object Reference"))
  (bind _asprimitive_component (cast `PrimitiveComponent` (`Actor.RootComponent` (`self.GetOwner`)))
    (:`then`
      (return _asprimitive_component))
    (:`CastFailed`
      (`KismetSystemLibrary.PrintString` "Error: No primitive component attached to root of ship AI."))))

(fn `SetTargetPosition`
  (params (NewTargetPosition :type "Vector Structure"))
  (set `self.TargetPosition` NewTargetPosition))

(fn `Update Line Trace Distance`
  (bind (_returnvalue_x _returnvalue_y _returnvalue_z) (`KismetMathLibrary.BreakVector` (`Actor.K2_GetActorLocation` (`GameplayStatics.GetPlayerCharacter` 0))))
  (if (> _returnvalue_z (`self.CheckGroundLineTraceDistance`))
    (set `self.LineTraceDistance` (+ _returnvalue_z (`KismetMathLibrary.RandomFloatInRange` 0.0 (`self.CheckGroundLineTraceDistanceRandomVariation`))))
    (else
      (set `self.LineTraceDistance` (`self.CheckGroundLineTraceDistance`)))))

(fn `ValidTargetPosition`
  (returns (TargetPositionValid :type Boolean))
  (return (!= (`self.TargetPosition`) (0.0 0.0 0.0))))