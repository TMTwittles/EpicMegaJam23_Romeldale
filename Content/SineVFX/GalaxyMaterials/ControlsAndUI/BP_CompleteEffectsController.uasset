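; Demo controller for GalaxyMaterials that steps through materials and effect actors with the E and Q keys.
; Each press applies the next or previous material to every slot on the listed actors, falling back to skeletal meshes when no static mesh exists.
; A parallel index spawns the matching effect class at the origin and destroys the previous one, starting on BeginPlay.
; Both indices wrap at hard-coded limits.
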(event `Key|E`
  (params (Key :type "Key Structure"))
  (bind _output (`|GetArrayItem` (`self.Materials`) (`self.CurrentMaterial`)))
  (:`Pressed`
    (bind _output_get (set `self.CurrentMaterial` (+ (`self.CurrentMaterial`) 1)))
    (`/Engine/EditorBlueprintResources/StandardMacros.CompareInt` _output_get 42
      (:`>`
        (set `self.CurrentMaterial` 0))
      (:`==`
        _)
      (:`<`
        _))
    (for _array_element (`self.StaticMeshActors`)
      (bind _returnvalue (`self.GetComponentByClass` _array_element "/Script/Engine.StaticMeshComponent"))
      (`/Engine/EditorBlueprintResources/StandardMacros.IsValid` _returnvalue
        (:`Is Valid`
          (for _index (range (`PrimitiveComponent.GetNumMaterials` _returnvalue))
            (`PrimitiveComponent.SetMaterial` _returnvalue _index _output)))
        (:`Is Not Valid`
          (bind _returnvalue_2 (`self.GetComponentByClass` _array_element "/Script/Engine.SkeletalMeshComponent"))
          (for _index_2 (range (`PrimitiveComponent.GetNumMaterials` _returnvalue_2))
            (`PrimitiveComponent.SetMaterial` _returnvalue_2 _index_2 _output)))))))

(event `Key|Q`
  (params (Key :type "Key Structure"))
  (bind _output (`|GetArrayItem` (`self.Materials`) (`self.CurrentMaterial`)))
  (:`Pressed`
    (bind _output_get (set `self.CurrentMaterial` (- (`self.CurrentMaterial`) 1)))
    (`/Engine/EditorBlueprintResources/StandardMacros.CompareInt` _output_get
      (:`>`
        _)
      (:`==`
        _)
      (:`<`
        (set `self.CurrentMaterial` 42)))
    (for _array_element (`self.StaticMeshActors`)
      (bind _returnvalue (`self.GetComponentByClass` _array_element "/Script/Engine.StaticMeshComponent"))
      (`/Engine/EditorBlueprintResources/StandardMacros.IsValid` _returnvalue
        (:`Is Valid`
          (for _index (range (`PrimitiveComponent.GetNumMaterials` _returnvalue))
            (`PrimitiveComponent.SetMaterial` _returnvalue _index _output)))
        (:`Is Not Valid`
          (bind _returnvalue_2 (`self.GetComponentByClass` _array_element "/Script/Engine.SkeletalMeshComponent"))
          (for _index_2 (range (`PrimitiveComponent.GetNumMaterials` _returnvalue_2))
            (`PrimitiveComponent.SetMaterial` _returnvalue_2 _index_2 _output)))))))

(event `Key|Q`
  (params (Key :type "Key Structure"))
  (:`Pressed`
    (bind _output_get (set `self.CurrentEffectInt` (+ (`self.CurrentEffectInt`) (* (`self.Int`) -1))))
    (`/Engine/EditorBlueprintResources/StandardMacros.CompareInt` _output_get -1
      (:`>`
        _)
      (:`==`
        (set `self.CurrentEffectInt` 42))
      (:`<`
        _))
    (bind _returnvalue (`|SpawnActorFromClass` (`|GetArrayItem` (`self.CompleteEffects`) (`self.CurrentEffectInt`)) (`KismetMathLibrary.MakeTransform` (0.0 0.0 0.0)) "Undefined" "OverrideRootScale" null null :!label _label))
    (`/Engine/EditorBlueprintResources/StandardMacros.IsValid` (`self.CurrentEffect`)
      (:`Is Valid`
        (set `self.PreviousEffect` (`self.CurrentEffect`))
        (set `self.CurrentEffect` _returnvalue)
        (`self.K2_DestroyActor` (`self.PreviousEffect`)))
      (:`Is Not Valid`
        (set `self.CurrentEffect` _returnvalue)))))

(event `Key|E`
  (params (Key :type "Key Structure"))
  (:`Pressed`
    (bind _output_get (set `self.CurrentEffectInt` (+ (`self.CurrentEffectInt`) (`self.Int`))))
    (`/Engine/EditorBlueprintResources/StandardMacros.CompareInt` _output_get 43
      (:`>`
        (goto _label))
      (:`==`
        (set `self.CurrentEffectInt` 0)
        (goto _label))
      (:`<`
        (goto _label)))))

(event `self.ReceiveBeginPlay`
  (`self.EnableInput` (`GameplayStatics.GetPlayerController` 0))
  (goto _label))

(fn `UserConstructionScript`)